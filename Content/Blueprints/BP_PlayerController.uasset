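; Player controller that creates the scoreboard widget and lets up to two fingers drag BP_PaddleActor paddles by touch.
; A touch press traces under the finger and grabs the hit paddle with that paddle's own physics handle, marking it Held.
; Tick moves each handle target to the finger's traced X and Y while keeping the paddle's Z.
; Releasing the touch drops the component and clears Held.
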(event EventBeginPlay
  (bind _returnvalue (UserInterface|CreateWidget "/Game/Blueprints/WBP/WBP_Scoreboard.WBP_Scoreboard_C"))
  (bind _output_get (Variables|Default|SetScoreboard _returnvalue))
  (UserInterface|Viewport|AddtoViewport _output_get 0))

(event EventTick
  (params (DeltaSeconds :type Float%20%28single-precision%29))
  (CallFunction|UpdatePaddleGrab (stale Input|TouchEvents|InputTouch _hitresult) (stale Input|TouchEvents|InputTouch _paddlephysicshandle) (stale Input|TouchEvents|InputTouch _fingerout))
  (CallFunction|UpdatePaddleGrab (stale Input|TouchEvents|InputTouch _hitresult_2) (stale Input|TouchEvents|InputTouch _paddlephysicshandle_2) (stale Input|TouchEvents|InputTouch _fingerout_2)))

(event Input|TouchEvents|InputTouch
  (params (Location :type Vector) (FingerIndex :type ETouchIndex%20Enum))
  ;[1 1 1] Relying on location rather than finger index would probably be more accurate. Current EndPaddleGrab isnt great
  (:Pressed
    (switch Utilities|FlowControl|Switch|SwitchonETouchIndex FingerIndex
      (:Touch1
        (bind (_hitresult _fingerout) (CallFunction|TouchPaddle "Touch1"))
        (bind _paddlephysicshandle (CallFunction|BeginPaddleGrab _hitresult)))
      (:Touch2
        (bind (_hitresult_2 _fingerout_2) (CallFunction|TouchPaddle "Touch2"))
        (bind _paddlephysicshandle_2 (CallFunction|BeginPaddleGrab _hitresult_2)))))
  (:Released
    (switch Utilities|FlowControl|Switch|SwitchonETouchIndex FingerIndex
      (:Touch1
        (CallFunction|EndPaddleGrab _hitresult _paddlephysicshandle))
      (:Touch2
        (CallFunction|EndPaddleGrab _hitresult_2 _paddlephysicshandle_2)))))

(fn ConstructionScript)

(fn TouchPaddle
  (params (Finger :type ETouchIndex%20Enum :default "Touch1"))
  (bind _hitresult (Class|PlayerController|GetHitResultUnderFingerbyChannel Finger "TraceTypeQuery1" true))
  (bind _hitactor (Collision|BreakHitResult _hitresult))
  (if (== (Utilities|GetClass _hitactor) "/Game/Blueprints/BP_PaddleActor.BP_PaddleActor_C")
    (Development|PrintString (Utilities|String|ToString(Text) (Utilities|Text|ToText(Object) _hitactor)) true true "(R=0.000000,G=1.000000,B=0.197686,A=1.000000)")
    (return _hitresult Finger)))

(fn BeginPaddleGrab
  (params (HitResult :type Hit%20Result%20Structure))
  (Utilities|IsValid (.hitactor HitResult)
    (:Is%20Valid
      (bind _asbp_paddle_actor (Utilities|Casting|CastToBP_PaddleActor (.hitactor HitResult)))
      (Physics|Components|PhysicsHandle|GrabComponentatLocationwithRotation (Variables|/Game/Blueprints/BP_PaddleActor.BP_PaddleActor_C|GetPhysicsHandle _asbp_paddle_actor) (.hitcomponent HitResult) "None" (.location HitResult) (Transformation|GetWorldRotation (Variables|/Script/Engine.Actor|GetRootComponent (CallFunction|GetGameModeBP))))
      (Variables|/Game/Blueprints/BP_PaddleActor.BP_PaddleActor_C|SetbHeld _asbp_paddle_actor true)
      (Development|PrintText (Utilities|Text|ToText(Object) (.hitactor HitResult)) true true "(R=1.000000,G=0.913103,B=0.062500,A=1.000000)")
      (return (Variables|/Game/Blueprints/BP_PaddleActor.BP_PaddleActor_C|GetPhysicsHandle _asbp_paddle_actor)))))

(fn EndPaddleGrab
  (params (HeldPaddle :type Hit%20Result%20Structure) (PaddlePhysicsHandle :type Physics%20Handle%20Component%20Object%20Reference))
  (Utilities|IsValid PaddlePhysicsHandle
    (:Is%20Valid
      (Utilities|IsValid (Class|PhysicsHandleComponent|GetGrabbedComponent PaddlePhysicsHandle)
        (:Is%20Valid
          (Physics|Components|PhysicsHandle|ReleaseComponent PaddlePhysicsHandle)
          (bind _asbp_paddle_actor (Utilities|Casting|CastToBP_PaddleActor (.hitactor HeldPaddle)))
          (Variables|/Game/Blueprints/BP_PaddleActor.BP_PaddleActor_C|SetbHeld _asbp_paddle_actor false)
          (Development|PrintText (Utilities|Text|ToText(Object) PaddlePhysicsHandle) true true "(R=1.000000,G=0.000000,B=0.094137,A=1.000000)"))))))

(fn UpdatePaddleGrab
  (params (HeldPaddle :type Hit%20Result%20Structure) (PaddlePhysicsHandle :type Physics%20Handle%20Component%20Object%20Reference) (Finger :type ETouchIndex%20Enum :default "Touch1"))
  (bind _hitresult (Class|PlayerController|GetHitResultUnderFingerbyChannel Finger "TraceTypeQuery1" true))
  (Utilities|IsValid PaddlePhysicsHandle
    (:Is%20Valid
      ;[1 1 1] A Cast on Tick is very inefficient. Need to setup call to event
      (bind _asbp_paddle_actor (Utilities|Casting|CastToBP_PaddleActor (.hitactor HeldPaddle)))
      (if (Variables|/Game/Blueprints/BP_PaddleActor.BP_PaddleActor_C|GetbHeld _asbp_paddle_actor)
        (Class|PhysicsHandleComponent|SetTargetLocationandRotation PaddlePhysicsHandle (Math|Vector|MakeVector (.x (.location _hitresult)) (.y (.location _hitresult)) (.z (Transformation|GetWorldLocation (Class|PhysicsHandleComponent|GetGrabbedComponent PaddlePhysicsHandle)))) "0, 0, 0")))))