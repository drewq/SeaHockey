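; BP_PuckActor is a physics puck that stays moving and is meant to change heading when stuck.
; Tick clamps the mesh's velocity to a minimum speed, saves its location and re-arms a GetPuckDirection timer every frame, restarting the countdown.
; GetPuckDirection randomizes mesh rotation if rounded X or Y matches the saved location.
; An older low-speed wander check using CustomEvent remains disconnected, and debug prints remain.
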(event Custom|CustomEvent
  ;[1 1 1] If the puck is going close to minimum speed for the duration of the timer, start to wander randomly
  (Development|PrintString "Hello")
  (bind _returnvalue (Physics|GetPhysicsLinearVelocity (Variables|Default|GetStaticMeshComp) "None"))
  (if (<= (Math|Vector|VectorLength _returnvalue) (Math|Vector|VectorLength (Variables|Default|GetTempVector)))
    (Transformation|SetRelativeRotation (Variables|Default|GetStaticMeshComp) (Math|Random|RandomRotator false) false false)))

(event Custom|GetPuckDirection
  (bind _staticmeshcomp (Variables|Default|GetStaticMeshComp))
  (bind _tempvector (Variables|Default|GetTempVector))
  (bind _returnvalue (Transformation|GetWorldLocation _staticmeshcomp))
  (Development|PrintString "Hello")
  (if (or (== (Math|Float|Round (.x _returnvalue)) (Math|Float|Round (.x _tempvector))) (== (Math|Float|Round (.y _returnvalue)) (Math|Float|Round (.y _tempvector))))
    (Transformation|SetRelativeRotation (Variables|Default|GetStaticMeshComp) (Math|Random|RandomRotator true) false false)))

(event EventBeginPlay)

(event Collision|EventActorBeginOverlap
  (params (OtherActor :type Actor%20Object%20Reference)))

(event EventTick
  (params (DeltaSeconds :type Float%20%28single-precision%29))
  (bind _staticmeshcomp (Variables|Default|GetStaticMeshComp))
  (bind _returnvalue (Physics|GetPhysicsLinearVelocity _staticmeshcomp "None"))
  (Physics|SetPhysicsLinearVelocity _staticmeshcomp (Math|Vector|ClampVectorSize _returnvalue 15.0 2e+06) false "None")
  (Variables|Default|SetTempVector (Transformation|GetWorldLocation _staticmeshcomp))
  (Utilities|Time|SetTimerbyEvent (delegate Custom|GetPuckDirection) 0.5))

(fn ConstructionScript)