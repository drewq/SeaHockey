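; Game mode for a puck-and-paddle team game that runs the match from setup to game over.
; On begin play it resets scores and spawns a puck at a random spawn point, plus one paddle per spawn point for two players or two for four.
; Goals credit the opposing team and update the scoreboard.
; The puck respawns after a short delay until either team hits the target score, opening the result menu.
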(event Custom|SpawnPuck
  (Game|SpawnActorfromClass "/Game/Blueprints/BP_PuckActor.BP_PuckActor_C" (.Transform (CallFunction|GetPuckSpawnPoint)) "AdjustIfPossibleButAlwaysSpawn" 0 0))

(event Custom|GameOver
  (Utilities|IsValid (Variables|Default|GetResultUI)
    (:Is%20Valid
      _)
    (:Is%20Not%20Valid
      (bind _returnvalue (UserInterface|CreateWidget "/Game/Blueprints/WBP/WBP_InGameMenu.WBP_InGameMenu_C"))
      (bind _output_get (Variables|Default|SetResultUI _returnvalue))))
  (UserInterface|Viewport|AddtoViewport _output_get 0))

(event Custom|SpawnPaddle
  (params (NumberOfPlayers :type Integer))
  (bind _paddlespawnactors (CallFunction|GetPaddleSpawnPoints))
  (switch int NumberOfPlayers
    (:2
      (for _array_element _paddlespawnactors
        (Game|SpawnActorfromClass "/Game/Blueprints/BP_PaddleActor.BP_PaddleActor_C" (Transformation|GetActorTransform _array_element) "AdjustIfPossibleButAlwaysSpawn" 0 0)))
    (:4
      (for _array_element_2 _paddlespawnactors
        (Game|SpawnActorfromClass "/Game/Blueprints/BP_PaddleActor.BP_PaddleActor_C" (Transformation|GetActorTransform _array_element_2) "AdjustIfPossibleButAlwaysSpawn" 0 0)
        (Game|SpawnActorfromClass "/Game/Blueprints/BP_PaddleActor.BP_PaddleActor_C" (Transformation|GetActorTransform _array_element_2) "AdjustIfPossibleButAlwaysSpawn" 0 0)))))

(event EventBeginPlay
  (Variables|Default|SetTeamOneScore 0)
  (Variables|Default|SetTeamTwoScore 0)
  (CallFunction|SpawnPuck)
  (CallFunction|SpawnPaddle (Variables|/Game/Blueprints/BP_GameInstance.BP_GameInstance_C|GetNumberOfPlayers (CallFunction|GetGameInstanceBP))))

(event EventTick
  (params (DeltaSeconds :type Float%20%28single-precision%29)))

(event EventOnGoalScored
  (params (GoalActor :type Actor%20Object%20Reference))
  (bind _mygameinstance (CallFunction|GetGameInstanceBP))
  (bind _gamecompletescore (Variables|/Game/Blueprints/BP_GameInstance.BP_GameInstance_C|GetGameCompleteScore _mygameinstance))
  (bind _asbp_goal_actor (Utilities|Casting|CastToBP_GoalActor GoalActor))
  (if (== (Class|SeaHockeyGoalActor|GetTeamNumber _asbp_goal_actor) 1)
    (CallFunction|TeamTwoScored)
    (else
      (CallFunction|TeamOneScored)))
  (if (or (== (Variables|Default|GetTeamOneScore) _gamecompletescore) (== (Variables|Default|GetTeamTwoScore) _gamecompletescore))
    (CallFunction|GameOver)
    (else
      (Utilities|FlowControl|Delay 0.5)
      (CallFunction|SpawnPuck))))

(fn ConstructionScript)

(fn TeamOneScored
  (bind _result (Math|Integer|IncrementInt (Variables|Default|GetTeamOneScore))
    (:%20%20
      (Default|UpdateScores (Variables|/Game/Blueprints/BP_PlayerController.BP_PlayerController_C|GetScoreboard (CallFunction|GetPlayerControllerBP)) 1 _result))))

(fn TeamTwoScored
  (bind _result (Math|Integer|IncrementInt (Variables|Default|GetTeamTwoScore))
    (:%20%20
      (Default|UpdateScores (Variables|/Game/Blueprints/BP_PlayerController.BP_PlayerController_C|GetScoreboard (CallFunction|GetPlayerControllerBP)) 2 _result))))

(fn GetPuckSpawnPoint
  (bind _outactors (Actor|GetAllActorsOfClass "/Game/Blueprints/BP_PuckSpawn.BP_PuckSpawn_C"))
  (if (Utilities|Array|IsValidIndex _outactors)
    (bind _output_get (LocalVariables|SetSpawnPoint (Transformation|GetActorTransform (Utilities|Array|Get(acopy) _outactors (Math|Random|RandomIntegerinRange 0 (Utilities|Array|LastIndex _outactors))))))
    (return true _output_get)
    (else
      (return (Utilities|Array|IsValidIndex _outactors) (LocalVariables|GetSpawnPoint)))))

(fn GetPaddleSpawnPoints
  (bind _outactors (Actor|GetAllActorsOfClass "/Game/Blueprints/BP_PaddleSpawn.BP_PaddleSpawn_C"))
  (if (Utilities|Array|IsValidIndex _outactors)
    (return true _outactors)
    (else
      (return (Utilities|Array|IsValidIndex _outactors) _outactors))))